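; Test AI enemy pawn that runs a behavior tree on BeginPlay, takes projectile damage and can hurt the player.
; Sphere overlaps accept three projectile types via a cast chain, converting Z scale (charge) into clamped damage.
; Each hit sets the combat state, plays explosion effects and destroys the projectile; the pawn is destroyed at zero health.
; Colliding with the first-person character hurts it only once, through an unreset DoOnce.
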(event OnComponentBeginOverlap(Sphere)
  (params (OverlappedComponent :type Primitive%20Component%20Object%20Reference) (OtherActor :type Actor%20Object%20Reference) (OtherComp :type Primitive%20Component%20Object%20Reference) (OtherBodyIndex :type Integer) (bFromSweep :type Boolean) (SweepResult :type Hit%20Result%20Structure%20%28by%20ref%29))
  (bind _returnvalue (Transformation|GetActorLocation))
  (bind _asfirst_person_projectile (Utilities|Casting|CastToFirstPersonProjectile OtherActor)
    (:then
      (Variables|Default|SetChargeScale (.z (Transformation|GetActorScale3D _asfirst_person_projectile))))
    (:CastFailed
      (bind _asfirst_person_projectile_yellow (Utilities|Casting|CastToFirstPersonProjectileYellow OtherActor)
        (:then
          (Variables|Default|SetChargeScale (.z (Transformation|GetActorScale3D _asfirst_person_projectile_yellow))))
        (:CastFailed
          (bind _asfirst_person_projectile_red (Utilities|Casting|CastToFirstPersonProjectileRed OtherActor))
          (Variables|Default|SetChargeScale (.z (Transformation|GetActorScale3D _asfirst_person_projectile_red)))))))
  (Variables|Default|SetCombatState (Utilities|Enum|LiteralenumENUM_AISTATE "NewEnumerator1"))
  (Effects|SpawnEmitteratLocation "/Game/StarterContent/Particles/P_Explosion.P_Explosion" _returnvalue)
  (Audio|PlaySoundatLocation "/Game/StarterContent/Audio/Explosion02.Explosion02" _returnvalue "0, 0, 0" 1.0 1.5 0.0 0 0 0)
  (Variables|Default|SetHealth (- (Variables|Default|GetHealth) (* (Math|Float|Clamp(Float) (Variables|Default|GetChargeScale) 1.0 5.0) 15.0)))
  (Development|PrintString (Utilities|String|ToString(Float) (* (Math|Float|Clamp(Float) (Variables|Default|GetChargeScale) 1.0 5.0) 15.0)))
  (Actor|DestroyActor _asfirst_person_projectile) ; Then destroy this projectile
  (if (<= (Variables|Default|GetHealth) 0.0)
    (Audio|PlaySoundatLocation "/Game/StarterContent/Audio/Explosion01.Explosion01" (Transformation|GetActorLocation self) "0, 0, 0" 2.0 1.0 0.0 0 0 0)
    (Actor|DestroyActor)))

(event EventBeginPlay
  (AI|RunBehaviorTree (AI|GetAIController self) "/Game/AI/BT_AIMainTest.BT_AIMainTest"))

(event Collision|EventActorBeginOverlap
  (params (OtherActor :type Actor%20Object%20Reference)))

(event Collision|EventHit
  (params (MyComp :type Primitive%20Component%20Object%20Reference) (Other :type Actor%20Object%20Reference) (OtherComp :type Primitive%20Component%20Object%20Reference) (bSelfMoved :type Boolean) (HitLocation :type Vector :default "0, 0, 0") (HitNormal :type Vector :default "0, 0, 0") (NormalImpulse :type Vector :default "0, 0, 0") (Hit :type Hit%20Result%20Structure%20%28by%20ref%29))
  (bind _asfirst_person_character (Utilities|Casting|CastToFirstPersonCharacter Other))
  (if (stale _bsuccess)
    (Utilities|FlowControl|DoOnce false
      (:Completed
        (Default|Hurt _asfirst_person_character 3e+01)
        (Development|PrintString "Hello")))))

(fn ConstructionScript)