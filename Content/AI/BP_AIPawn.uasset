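; BP_AIPawn is an enemy pawn that runs BT_AIMain and fights the player.
; Player projectile hits set its combat state, deal damage scaled by projectile size as charge, and at zero health it drops BP_Heal.
; Shoot starts a looping timer that fires projectiles toward the player at random speed while CombatState allows.
; Touching its Box hurts and launches the player, with a short cooldown.
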(event `self.ReceiveBeginPlay`
  (`AIController.RunBehaviorTree` (`AIBlueprintHelperLibrary.GetAIController` self) "/Game/AI/BT_AIMain.BT_AIMain"))

(event `self.Hitbox.OnComponentBeginOverlap`
  (params (OverlappedComponent :type "PrimitiveComponent Object Reference") (OtherActor :type "Actor Object Reference") (OtherComp :type "PrimitiveComponent Object Reference") (OtherBodyIndex :type Integer) (bFromSweep :type Boolean) (SweepResult :type "HitResult Structure (by ref)"))
  (bind _returnvalue (`self.K2_GetActorLocation`))
  (bind _asfirst_person_projectile (cast `/Game/FirstPersonBP/Blueprints/FirstPersonProjectile` OtherActor)
    (:`then`
      (bind (_returnvalue_x _returnvalue_y _returnvalue_z) (`KismetMathLibrary.BreakVector` (`self.GetActorScale3D` _asfirst_person_projectile)))
      (set `self.ChargeScale` _returnvalue_z))
    (:`CastFailed`
      (bind _asfirst_person_projectile_yellow (cast `/Game/FirstPersonBP/Blueprints/FirstPersonProjectileYellow` OtherActor)
        (:`then`
          (bind (_returnvalue_x_2 _returnvalue_y_2 _returnvalue_z_2) (`KismetMathLibrary.BreakVector` (`self.GetActorScale3D` _asfirst_person_projectile_yellow)))
          (set `self.ChargeScale` _returnvalue_z_2))
        (:`CastFailed`
          (bind _asfirst_person_projectile_red (cast `/Game/FirstPersonBP/Blueprints/FirstPersonProjectileRed` OtherActor))
          (bind (_returnvalue_x_3 _returnvalue_y_3 _returnvalue_z_3) (`KismetMathLibrary.BreakVector` (`self.GetActorScale3D` _asfirst_person_projectile_red)))
          (set `self.ChargeScale` _returnvalue_z_3)))))
  (set `self.Combat State` (enumliteral `/Game/AI/ENUM_AISTATE` "NewEnumerator1"))
  (`GameplayStatics.SpawnEmitterAtLocation` "/Game/StarterContent/Particles/P_Explosion.P_Explosion" _returnvalue)
  (`GameplayStatics.PlaySoundAtLocation` "/Game/StarterContent/Audio/Explosion02.Explosion02" _returnvalue (struct) 1.0 1.5 0.0 null null null)
  (set `self.Health` (- (`self.Health`) (* (`KismetMathLibrary.FClamp` (`self.ChargeScale`) 1.0 5.0) 15.0)))
  (`self.K2_DestroyActor` _asfirst_person_projectile)
  (`self.K2_DestroyActor` _asfirst_person_projectile_yellow) ; Then destroy this projectile
  (if (<= (`self.Health`) 0.0)
    (`GameplayStatics.PlaySoundAtLocation` "/Game/StarterContent/Audio/Explosion01.Explosion01" (`self.K2_GetActorLocation` self) (struct) 2.0 1.0 0.0 null null null)
    (`|SpawnActorFromClass` "/Game/FirstPersonBP/Blueprints/BP_Heal.BP_Heal_C" (`KismetMathLibrary.MakeTransform` (`self.K2_GetActorLocation` self)) "AlwaysSpawn" "OverrideRootScale" null null)
    (`self.K2_DestroyActor`)))

(event `Shoot`
  (bind _returnvalue (`self.K2_GetActorLocation` self))
  (`/Engine/EditorBlueprintResources/StandardMacros.DoOnce` false :!label _label
    (:`Completed`
      (set `self.isLoopingBullets` true)
      (`KismetSystemLibrary.K2_SetTimerDelegate` (delegate `ShootBullet`) 1.5 (`self.isLoopingBullets`))
      (`/Engine/EditorBlueprintResources/StandardMacros.DoOnce` false :!via `Reset`
        (:`Completed`
          (bind _returnvalue_2 (`|SpawnActorFromClass` "/Game/FirstPersonBP/Blueprints/AI_Projectile_Test.AI_Projectile_Test_C" (`KismetMathLibrary.MakeTransform` (`self.K2_GetActorLocation` self)) "AlwaysSpawn" "OverrideRootScale" null null :!label _label_2))
          (`GameplayStatics.SpawnSoundAtLocation` "/Game/Audio/Sci-fi__Weapon__Blaster__Laser__Boom__Heavy_6_SND7297.Sci-fi__Weapon__Blaster__Laser__Boom__Heavy_6_SND7297" _returnvalue (struct) 0.2 1.0 0.0 "/Game/Audio/ExplosionAtten.ExplosionAtten" null)
          (set `MovementComponent.Velocity` (* (- (`self.K2_GetActorLocation` (`GameplayStatics.GetPlayerCharacter` 0)) _returnvalue) (`KismetMathLibrary.FClamp` (`KismetMathLibrary.RandomFloat`) 0.5)) (`/Game/FirstPersonBP/Blueprints/AI_Projectile_Test.Projectile` _returnvalue_2)))))))

(event `TakeDamage`
  (params (Damage :type "Float (double-precision)"))
  (set `self.Health` (- (`self.Health`) Damage)))

(event `ShootBullet`
  (if (`|EnumEquality` (`self.Combat State`) "NewEnumerator2")
    (set `self.isLoopingBullets` true)
    (goto _label_2)
    (else
      (set `self.isLoopingBullets` false)
      (goto _label :!via `Reset`))))

(event `CheckHealth`
  (if (<= (`self.Health`) 0.0)
    (`|SpawnActorFromClass` "/Game/FirstPersonBP/Blueprints/BP_Heal.BP_Heal_C" (`KismetMathLibrary.MakeTransform` (`self.K2_GetActorLocation` self)) "AlwaysSpawn" "OverrideRootScale" null null)
    (`self.K2_DestroyActor`)))

(event `self.Box.OnComponentBeginOverlap`
  (params (OverlappedComponent :type "PrimitiveComponent Object Reference") (OtherActor :type "Actor Object Reference") (OtherComp :type "PrimitiveComponent Object Reference") (OtherBodyIndex :type Integer) (bFromSweep :type Boolean) (SweepResult :type "HitResult Structure (by ref)"))
  (bind (_returnvalue_x _returnvalue_y) (`KismetMathLibrary.BreakVector` (* (`self.GetActorForwardVector` self) 500)))
  (bind _asfirst_person_character (cast `/Game/FirstPersonBP/Blueprints/FirstPersonCharacter` OtherActor))
  (`/Engine/EditorBlueprintResources/StandardMacros.DoOnce` false :!label _label_3
    (:`Completed`
      (`/Game/FirstPersonBP/Blueprints/FirstPersonCharacter.Hurt` _asfirst_person_character 10.0)
      (`self.LaunchCharacter` _asfirst_person_character (`KismetMathLibrary.MakeVector` _returnvalue_x _returnvalue_y 500.0) true true)
      (`KismetSystemLibrary.Delay` 2.0)
      (goto _label_3 :!via `Reset`))))

(fn `UserConstructionScript`)