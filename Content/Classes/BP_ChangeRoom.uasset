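; BP_ChangeRoom is a trigger actor that records which room the first-person player has entered.
; When the character overlaps its Box, it writes RoomToGoTo into CurrentRoomNumber on BP_GameManager.
; If the room differs from the current one, it also calls UpdateRoom on BP_MapCamera_Main, finding both actors by class lookup.
; Unconnected leftovers include a room-number switch, wind-volume ambience timelines and a DoOnce delay.
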(event `self.Box.OnComponentBeginOverlap`
  (params (OverlappedComponent :type "PrimitiveComponent Object Reference") (OtherActor :type "Actor Object Reference") (OtherComp :type "PrimitiveComponent Object Reference") (OtherBodyIndex :type Integer) (bFromSweep :type Boolean) (SweepResult :type "HitResult Structure (by ref)"))
  (bind _roomtogoto (`self.RoomToGoTo`))
  (cast `/Game/FirstPersonBP/Blueprints/FirstPersonCharacter` OtherActor)
  (bind _outactors (`GameplayStatics.GetAllActorsOfClass` "/Game/Classes/BP_GameManager.BP_GameManager_C"))
  (bind _output (`|GetArrayItem` _outactors))
  (if (== (`self.RoomToGoTo`) (`/Game/Classes/BP_GameManager.CurrentRoomNumber` _output))
    (set `/Game/Classes/BP_GameManager.CurrentRoomNumber` _roomtogoto _output)
    (else
      (set `/Game/Classes/BP_GameManager.CurrentRoomNumber` _roomtogoto _output)
      (bind _outactors_2 (`GameplayStatics.GetAllActorsOfClass` "/Game/Classes/BP_MapCamera_Main.BP_MapCamera_Main_C"))
      (`/Game/Classes/BP_MapCamera_Main.UpdateRoom` (`|GetArrayItem` _outactors_2)))))

(fn `UserConstructionScript`)