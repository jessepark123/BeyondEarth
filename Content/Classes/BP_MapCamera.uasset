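; BP_MapCamera is a map camera actor that mirrors the player on a scaled-down map and highlights the current room.
; Each Tick it moves a Player marker from the pawn's scaled location and matches the spring arm to pawn yaw and roll at fixed pitch.
; It polls BP_GameManager's CurrentRoomNumber to swap two room materials and snap the spring arm to that room's point.
; The GoToRoom0 timeline blend is left unused.
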(event `self.ReceiveTick`
  (params (DeltaSeconds :type "Float (single-precision)"))
  (bind _returnvalue (`GameplayStatics.GetPlayerPawn` 0))
  (bind _springarm (`self.SpringArm`))
  (bind _room0 (`self.Room0`))
  (bind _room1 (`self.Room1`))
  (bind (_returnvalue_roll _returnvalue_pitch _returnvalue_yaw) (`KismetMathLibrary.BreakRotator` (`self.K2_GetActorRotation` _returnvalue)))
  (bind (_returnvalue_x _returnvalue_y _returnvalue_z) (`KismetMathLibrary.BreakVector` (`self.K2_GetActorLocation` _returnvalue)))
  (`SceneComponent.K2_SetRelativeLocation` (`self.Player`) (/ (`self.K2_GetActorLocation` (`GameplayStatics.GetPlayerPawn` 0)) (15.0 15.0 3.0)) false false)
  (`SceneComponent.K2_SetWorldRotation` _springarm (`KismetMathLibrary.MakeRotator` _returnvalue_roll -30.0 _returnvalue_yaw) false false)
  (`SceneComponent.K2_SetRelativeLocation` _springarm (`KismetMathLibrary.MakeVector` 0.0 0.0 (- _returnvalue_z 60.0)) false false)
  (bind _outactors (`GameplayStatics.GetAllActorsOfClass` "/Game/Classes/BP_GameManager.BP_GameManager_C"))
  (switch `int` (`/Game/Classes/BP_GameManager.CurrentRoomNumber` (cast `/Game/Classes/BP_GameManager` (`|GetArrayItem` _outactors) :!pure true))
    (:`0`
      (`PrimitiveComponent.SetMaterial` _room0 0 "/Game/Geometry/Meshes/CubeMaterial.CubeMaterial")
      (`PrimitiveComponent.SetMaterial` _room1 0 "/Game/Geometry/Meshes/CubeMaterial_Unselected.CubeMaterial_Unselected")
      (`SceneComponent.K2_SetWorldLocation` _springarm (`SceneComponent.K2_GetComponentLocation` (`self.0`)) false false)
      (`SceneComponent.K2_SetWorldLocation` (`self.SpringArm`) (`SceneComponent.K2_GetComponentLocation` (`self.0`)) false false))
    (:`1`
      (`PrimitiveComponent.SetMaterial` _room1 0 "/Game/Geometry/Meshes/CubeMaterial.CubeMaterial")
      (`PrimitiveComponent.SetMaterial` _room0 0 "/Game/Geometry/Meshes/CubeMaterial_Unselected.CubeMaterial_Unselected")
      (`SceneComponent.K2_SetWorldLocation` (`self.SpringArm`) (`SceneComponent.K2_GetComponentLocation` (`self.1`)) false false))))

(event `MovePawn`
  (params (Direction :type "Vector Structure") (ScaleValue :type "Float (double-precision)")))

(fn `UserConstructionScript`)