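; Shootable rock actor that moves only when hit by the projectile type matching its ShootMat material, which the construction script applies to StaticMesh1.
; Each valid Box overlap plays a sound and toggles between playing the MoveRock timeline from the start and stopping it.
; The timeline adds swept vertical offsets to Rock, scaled by DistanceToFall.
; StaticMesh1 hides while the rock moves and reappears when a hit stops it.
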(event `RockFall`
  (bind (_direction _translation) (`Timeline|MoveRock` :!via `PlayFromStart` :!label _label)
    (:`Update`
      (`SceneComponent.K2_AddRelativeLocation` (`self.Rock`) (`KismetMathLibrary.MakeVector` 0.0 0.0 (* _translation (`self.Distance_toFall`))) true false))
    (:`Finished`
      _))
  (`SceneComponent.SetVisibility` (`self.StaticMesh1`) (not (stale `self.Box.OnComponentBeginOverlap` _isa)) false :!label _label_2))

(event `self.Box.OnComponentBeginOverlap`
  (params (OverlappedComponent :type "PrimitiveComponent Object Reference") (OtherActor :type "Actor Object Reference") (OtherComp :type "PrimitiveComponent Object Reference") (OtherBodyIndex :type Integer) (bFromSweep :type Boolean) (SweepResult :type "HitResult Structure (by ref)"))
  (if (== (`self.ShootMat`) "/Engine/VREditor/BasicMeshes/MI_Cube_01.MI_Cube_01")
    (cast `/Game/FirstPersonBP/Blueprints/FirstPersonProjectileYellow` OtherActor)
    (`GameplayStatics.PlaySound2D` "/Game/Audio/Sci-fi__Spark__Electric_Device__Hum_1_SND7085.Sci-fi__Spark__Electric_Device__Hum_1_SND7085" 1.0 1.2 0.0 null null :!label _label_3)
    (bind _isa (`/Engine/EditorBlueprintResources/StandardMacros.FlipFlop`)
      (:`A`
        _)
      (:`B`
        _))
    (bind _output_get (set `self.isMovable` _isa))
    (if _output_get
      (`self.RockFall`)
      (else
        (`|ExecutionSequence`
          (:`then_0`
            (goto _label_2))
          (:`then_1`
            (goto _label :!via `Stop`)))))
    (elif (== (`self.ShootMat`) "/Engine/VREditor/BasicMeshes/MI_Cube_03.MI_Cube_03")
      (cast `/Game/FirstPersonBP/Blueprints/FirstPersonProjectileRed` OtherActor)
      (goto _label_3)
      (elif (== (`self.ShootMat`) "/Engine/VREditor/BasicMeshes/MI_Cube_02.MI_Cube_02")
        (cast `/Game/FirstPersonBP/Blueprints/FirstPersonProjectile` OtherActor)
        (goto _label_3)))))

(fn `UserConstructionScript`
  (`PrimitiveComponent.SetMaterial` (`self.StaticMesh1`) 0 (`self.ShootMat`)))