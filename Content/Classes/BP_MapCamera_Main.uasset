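; Map camera actor that shows the player's position and current room on a scaled-down map.
; Each tick it places a Player marker from scaled pawn coordinates and turns the spring arm with the pawn's yaw at fixed pitch.
; BP_GameManager's CurrentRoomNumber selects the highlighted material slot and whether the arm centers on a room anchor or the marker.
; UpdateRoom resets a DoOnce so the next tick clears old highlights.
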(event `self.ReceiveTick`
  (params (DeltaSeconds :type "Float (single-precision)"))
  (bind _returnvalue (`GameplayStatics.GetPlayerPawn` 0))
  (bind _springarm (`self.SpringArm`))
  (bind _player (`self.Player`))
  (bind (_returnvalue_roll _returnvalue_pitch _returnvalue_yaw) (`KismetMathLibrary.BreakRotator` (`self.K2_GetActorRotation` _returnvalue)))
  (bind (_returnvalue_x _returnvalue_y _returnvalue_z) (`KismetMathLibrary.BreakVector` (`self.K2_GetActorLocation` _returnvalue)))
  (`SceneComponent.K2_SetRelativeLocation` (`self.Player`) (/ (`self.K2_GetActorLocation` (`GameplayStatics.GetPlayerPawn` 0)) (3.95 3.95 3.5)) false false)
  (`SceneComponent.K2_SetWorldRotation` _springarm (`KismetMathLibrary.MakeRotator` _returnvalue_roll -30.0 _returnvalue_yaw) false false)
  (`SceneComponent.K2_SetRelativeLocation` _springarm (`KismetMathLibrary.MakeVector` 0.0 0.0 (- _returnvalue_z 60.0)) false false)
  (bind _outactors (`GameplayStatics.GetAllActorsOfClass` "/Game/Classes/BP_GameManager.BP_GameManager_C"))
  (`|ExecutionSequence`
    (:`then_0`
      (`/Engine/EditorBlueprintResources/StandardMacros.DoOnce` false :!label _label
        (:`Completed`
          (for _index (range 17)
            (`PrimitiveComponent.SetMaterial` (`self.Map`) _index "/Game/Geometry/Meshes/CubeMaterial_Unselected.CubeMaterial_Unselected")))))
    (:`then_1`
      (bind _currentroomnumber (`/Game/Classes/BP_GameManager.CurrentRoomNumber` (`|GetArrayItem` _outactors)))
      (`PrimitiveComponent.SetMaterial` (`self.Map`) _currentroomnumber "/Game/Geometry/Meshes/CubeMaterial.CubeMaterial"))
    (:`then_2`
      (switch `int` _currentroomnumber
        (:`0`
          (`SceneComponent.K2_SetWorldLocation` (`self.SpringArm`) (`SceneComponent.K2_GetComponentLocation` (`self.Room0`)) false false))
        (:`1`
          (`SceneComponent.K2_SetWorldLocation` (`self.SpringArm`) (`SceneComponent.K2_GetComponentLocation` (`self.Room1`)) false false))
        (:`2`
          (`SceneComponent.K2_SetWorldLocation` (`self.SpringArm`) (`SceneComponent.K2_GetComponentLocation` (`self.Player`)) false false :!label _label_2))
        (:`3`
          (`SceneComponent.K2_SetWorldLocation` (`self.SpringArm`) (`SceneComponent.K2_GetComponentLocation` (`self.Room3`)) false false))
        (:`4`
          (`SceneComponent.K2_SetWorldLocation` (`self.SpringArm`) (`SceneComponent.K2_GetComponentLocation` _player) false false :!label _label_3)
          (`PrimitiveComponent.SetMaterial` (`self.Map`) 15 "/Game/Geometry/Meshes/CubeMaterial.CubeMaterial"))
        (:`5`
          (`SceneComponent.K2_SetWorldLocation` (`self.SpringArm`) (`SceneComponent.K2_GetComponentLocation` _player) false false))
        (:`6`
          (`SceneComponent.K2_SetWorldLocation` (`self.SpringArm`) (`SceneComponent.K2_GetComponentLocation` (`self.Room6`)) false false))
        (:`7`
          (`SceneComponent.K2_SetWorldLocation` (`self.SpringArm`) (`SceneComponent.K2_GetComponentLocation` (`self.Room7`)) false false))
        (:`8`
          (`SceneComponent.K2_SetWorldLocation` (`self.SpringArm`) (`SceneComponent.K2_GetComponentLocation` (`self.Room8`)) false false))
        (:`9`
          (`SceneComponent.K2_SetWorldLocation` (`self.SpringArm`) (`SceneComponent.K2_GetComponentLocation` (`self.Player`)) false false))
        (:`10`
          (`SceneComponent.K2_SetWorldLocation` (`self.SpringArm`) (`SceneComponent.K2_GetComponentLocation` (`self.Player`)) false false))
        (:`11`
          (`SceneComponent.K2_SetWorldLocation` (`self.SpringArm`) (`SceneComponent.K2_GetComponentLocation` (`self.Room11`)) false false :!label _label_4)
          (`PrimitiveComponent.SetMaterial` (`self.Map`) 13 "/Game/Geometry/Meshes/CubeMaterial.CubeMaterial"))
        (:`12`
          (`SceneComponent.K2_SetWorldLocation` (`self.SpringArm`) (`SceneComponent.K2_GetComponentLocation` (`self.Room12`)) false false))
        (:`13`
          (goto _label_4))
        (:`14`
          (goto _label_2))
        (:`15`
          (goto _label_3))))))

(event `UpdateRoom`
  (goto _label :!via `Reset`))

(fn `UserConstructionScript`)